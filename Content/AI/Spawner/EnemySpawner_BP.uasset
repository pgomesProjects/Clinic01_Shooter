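; Enemy spawner actor that spawns batches of enemies at its own transform, starting when play begins.
; BeginPlay calls the SpawnEnemy event with the Enemy, transform and NumberOfEnemies values, and the event spawns that many actors in a loop.
; After each batch it waits SpawnDelay, then calls itself with the actor's current transform, repeating with no stop condition.
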(event `self.ReceiveBeginPlay`
  ;[1 1 1] Spawn Enemies At Start
  (`self.SpawnEnemy` (`self.Enemy`) (`self.GetTransform`) (`self.Number Of Enemies`)))

(event `SpawnEnemy`
  (params (Enemy :type "Actor Class Reference") (SpawnTransform :type "Transform Structure") (NumberOfEnemies :type Integer))
  ;[1 1 1] Spawn In A Number Of Enemies And Delay Before Doing It Again
  (for _ (range NumberOfEnemies)
    (`|SpawnActorFromClass` "/Game/AI/Enemy.Enemy_C" SpawnTransform "Undefined" "OverrideRootScale" null null))
  (`KismetSystemLibrary.Delay` (`self.SpawnDelay`))
  (`self.SpawnEnemy` (`self.Enemy`) (`self.GetTransform`) (`self.Number Of Enemies`)))

(fn `UserConstructionScript`)